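; Game mode for a drone and turrets game that manages the HUD and end-of-game screen.
; GameStart creates the ammo and HP widgets and adds them to the viewport.
; GameOver shows a game-over widget with win or lose text chosen by its WonGame flag, then removes both HUD widgets.
; Neither event is called within this Blueprint, and BeginPlay and Tick are unused stubs.
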(event EventBeginPlay)

(event EventTick
  (params (DeltaSeconds :type Float%20%28single-precision%29)))

(event EventGameOver
  (params (bWonGame :type Boolean))
  (if bWonGame
    _
    (else
      _))
  (bind _returnvalue (UserInterface|CreateWidget "/Game/Blueprints/Widgets/BP_GameOver.BP_GameOver_C"))
  (UserInterface|Viewport|AddtoViewport _returnvalue 0)
  (Variables|/Script/UMG.TextBlock|SetText (Variables|/Game/Blueprints/Widgets/BP_GameOver.BP_GameOver_C|GetTEXT_GameOver _returnvalue) (select bWonGame "You win" "You lose"))
  (Widget|RemovefromParent (stale EventGameStart _returnvalue)))

(event EventGameStart
  (bind _returnvalue (UserInterface|CreateWidget "/Game/Blueprints/Widgets/BP_Ammo.BP_Ammo_C"))
  (UserInterface|Viewport|AddtoViewport _returnvalue 0)
  (bind _returnvalue_2 (UserInterface|CreateWidget "/Game/Blueprints/Widgets/BP_HPWidget.BP_HPWidget_C"))
  (UserInterface|Viewport|AddtoViewport _returnvalue_2 0))

(fn ConstructionScript)